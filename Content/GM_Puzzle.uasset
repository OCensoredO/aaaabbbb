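; GM_Puzzle is a puzzle game mode Blueprint that runs startup setup and debug output on BeginPlay.
; It calls GMPlayerDie immediately, adds BP_Widget to the viewport and prints HP.
; It then reads DT_GameData by numeric row names from 1 to the row count, printing each row's name, HP, gossip and image.
; An unconnected legacy block holds old HP increment and update logic.
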(event `self.ReceiveBeginPlay`
  (`|ExecutionSequence`
    (:`then_0`
      (`self.GM_Player_Die`)
      (`KismetSystemLibrary.PrintString` "Hello")
      (bind _returnvalue (`|CreateWidget` "/Game/BP_Widget.BP_Widget_C"))
      (`UserWidget.AddToViewport` _returnvalue 0)
      (`KismetSystemLibrary.PrintString` (`KismetStringLibrary.Conv_IntToString` (`self.HP`)) true true (struct :`G` 0.66 :`B` 1.0 :`A` 1.0) 12.0))
    (:`then_2`
      ;[1 1 1] Data Table 길이 얻어오기
      (bind _outrownames (`DataTableFunctionLibrary.GetDataTableRowNames` "/Game/DT_GameData.DT_GameData"))
      (set `self.DataTableLength` (`KismetArrayLibrary.Array_Length` _outrownames)))
    (:`then_3`
      ;[1 1 1] Data Table 데이터 추출
      (for _index (range 1 (+ (`self.DataTableLength`) 1))
        (bind _returnvalue_2 (`|GetDataTableRow` "/Game/DT_GameData.DT_GameData" (`KismetStringLibrary.Conv_StringToName` (`KismetStringLibrary.Conv_IntToString` _index)))
          (:`then`
            (bind (_name _hp _gossip _image) (break `/Game/ST_GameChatData` _returnvalue_2))
            (`KismetSystemLibrary.PrintString` (`KismetTextLibrary.Conv_TextToString` (`|FormatText` "Name : {0}, HP : {1}, Gossip : {2}, Image : {3}" _name _hp _gossip _image)))))))))

(event `self.ReceiveTick`
  (params (DeltaSeconds :type "Float (single-precision)")))

(fn `UserConstructionScript`)